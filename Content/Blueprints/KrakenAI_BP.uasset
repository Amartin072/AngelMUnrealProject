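; Kraken enemy AI that roams to random reachable points and chases pawns it senses, playing a short-range attack montage on arrival.
; The first chase triggers a cutscene that blends the player's camera to the Kraken and locks input to UI.
; Tick drives chasing, a player-facing health bar, fleeing at low health and delayed destruction at zero.
; A timer regenerates health, and overlapping the player subtracts player health.
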(event `self.ReceiveTick`
  (params (DeltaSeconds :type "Float (single-precision)"))
  ; TickEvent
  (`self.UpdatePawnChase`)
  (`self.UpdateHealthBar`)
  (`self.CheckHealth`))

(event `self.ReceiveBeginPlay`
  ; BeginPlay
  (`self.Roam`)
  (`KismetSystemLibrary.K2_SetTimer` null "RegenHealth" 10.0 true))

(event `Roam`
  ; Roam
  (if (`self.IsPlayingCinematic`)
    _
    (elif (`self.IsDead`)
      _
      (elif (`self.IsFleeing`)
        _
        (elif (`self.IsRoaming`)
          _
          (elif (not (`self.IsAttacking`))
            (set `self.IsRoaming` true)
            (`|AIMoveTo` self (`NavigationSystemV1.K2_GetRandomReachablePointInRadius` (`self.K2_GetActorLocation`) 3000.0 null null) null 250.0
              (:`OnSuccess`
                _)
              (:`OnFail`
                _))
            (`KismetSystemLibrary.Delay` 5.0)
            (set `self.IsRoaming` false)
            (`self.Roam`)))))))

(event `self.PawnSensing.OnSeePawn`
  (params (Pawn :type "Pawn Object Reference"))
  ; Event -- Pawn Chase
  (set `self.ChasingPawn` Pawn))

(event `UpdatePawnChase`
  ; Update Pawn Chase
  (`/Engine/EditorBlueprintResources/StandardMacros.IsValid` (`self.ChasingPawn`)
    (:`Is Valid`
      (if (< (`KismetMathLibrary.Vector_Distance` (`self.K2_GetActorLocation` (`self.ChasingPawn`)) (`self.K2_GetActorLocation`)) 2500.0)
        (if (`self.IsPlayingCinematic`)
          (`Controller.StopMovement` (`AIBlueprintHelperLibrary.GetAIController` self))
          (elif (`self.IsFleeing`)
            _
            (elif (`self.IsDead`)
              _
              (elif (not (`self.IsAttacking`))
                (set `self.IsAttacking` true)
                (`Controller.StopMovement` (`AIBlueprintHelperLibrary.GetAIController` self))
                (if (`self.IsFirstChase`)
                  (set `self.IsFirstChase` false)
                  (`self.FirstChaseCinematic`))
                (`|AIMoveTo` self (0.0 0.0 0.0) (`self.ChasingPawn`) 1200.0
                  (:`OnSuccess`
                    (bind _returnvalue (`self.PlayAnimMontage` "/Game/Blueprints/ShortRangeAttack_Montage.ShortRangeAttack_Montage"))
                    (`KismetSystemLibrary.Delay` _returnvalue))
                  (:`OnFail`
                    _))
                (set `self.IsAttacking` false)
                (`self.Roam`)))))))
    (:`Is Not Valid`
      (`self.Roam`))))

(event `UpdateHealthBar`
  ; Update Health Bar
  (`SceneComponent.K2_SetWorldRotation` (`self.HealthBar`) (`KismetMathLibrary.FindLookAtRotation` (`self.K2_GetActorLocation`) (`self.K2_GetActorLocation` (`GameplayStatics.GetPlayerCharacter` 0))) false false)
  (bind _askraken_health_bp (cast `/Game/Blueprints/KrakenHealth_BP` (`WidgetComponent.GetWidget` (`self.HealthBar`))))
  (`ProgressBar.SetPercent` (`/Game/Blueprints/KrakenHealth_BP.ProgressBar_48` _askraken_health_bp) (/ (`self.Health`) (`self.MaxHealth`))))

(event `CheckHealth`
  ; Check Health / Death
  (if (<= (`self.Health`) 0)
    (set `self.IsDead` true)
    (`Controller.StopMovement` (`AIBlueprintHelperLibrary.GetAIController` self))
    (`KismetSystemLibrary.Delay` 10.0)
    (`self.K2_DestroyActor`)
    (elif (<= (`self.Health`) (`self.FleeingHealthThreshold`))
      (`self.RunAway`)
      (else
        (set `self.IsFleeing` false)))))

(event `RunAway`
  (bind _returnvalue (`self.K2_GetActorLocation`))
  ; Run Away
  (if (not (`self.IsFleeing`))
    (set `self.IsFleeing` true)
    (`|AIMoveTo` self (`NavigationSystemV1.K2_GetRandomReachablePointInRadius` (`KismetMathLibrary.MakeVector` (.x (+ _returnvalue (* (`KismetMathLibrary.GetForwardVector` (`KismetMathLibrary.FindLookAtRotation` _returnvalue (`self.K2_GetActorLocation` (`self.ChasingPawn`)))) -500))) (.y (+ _returnvalue (* (`KismetMathLibrary.GetForwardVector` (`KismetMathLibrary.FindLookAtRotation` _returnvalue (`self.K2_GetActorLocation` (`self.ChasingPawn`)))) -500))) (.z _returnvalue)) 500.0 null null) null 200.0
      (:`OnSuccess`
        _)
      (:`OnFail`
        _))
    (set `self.IsFleeing` false)))

(event `FirstChaseCinematic`
  (bind _returnvalue (`GameplayStatics.GetPlayerController` 0))
  ; Battle Start Cutscene
  (if (not (`self.IsPlayingCinematic`))
    (set `self.IsPlayingCinematic` true)
    (`Controller.StopMovement` (`AIBlueprintHelperLibrary.GetAIController` self))
    (`WidgetBlueprintLibrary.SetInputMode_UIOnlyEx` _returnvalue null)
    (`PlayerController.SetViewTargetWithBlend` _returnvalue self 0.5 "VTBlend_Linear" 0.0 false)
    (bind _returnvalue_2 (`self.PlayAnimMontage` "/Game/Blueprints/FirstChase_Montage.FirstChase_Montage"))
    (`KismetSystemLibrary.Delay` _returnvalue_2)
    (`PlayerController.SetViewTargetWithBlend` _returnvalue (`self.ChasingPawn`) 0.5 "VTBlend_Linear" 0.0 false)
    (`WidgetBlueprintLibrary.SetInputMode_GameOnly` _returnvalue)
    (`KismetSystemLibrary.Delay` 2.0)
    (set `self.IsPlayingCinematic` false)))

(event `self.ReceiveActorBeginOverlap`
  (params (OtherActor :type "Actor Object Reference"))
  (bind _asbp_player (cast `/Game/BP_Player` OtherActor))
  (bind _output_get (set `/Game/BP_Player.Player Health` (- (`/Game/BP_Player.Player Health` _asbp_player) 25) _asbp_player))
  (`KismetSystemLibrary.PrintString` (`KismetStringLibrary.Conv_IntToString` _output_get)))

(fn `RegenHealth`
  (if (< (`self.Health`) (`self.MaxHealth`))
    (set `self.Health` (+ (`self.Health`) (`self.HealthRegenRate`)))))

(fn `UserConstructionScript`)